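; BP_Platform is a launch pad that rewards or penalizes BP_Pawn based on whether its material matches the platform's.
; The construction script picks a random shape form, which BeginPlay turns into a material and impact sound.
; On overlap, a match launches the pawn along the pitch-adjusted facing and adds score through BP_GameMode.
; A mismatch flips the direction with random force and subtracts score, each outcome with its own VFX and sound.
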(event Custom|LaunchProper
  (params (Target :type Character%20Object%20Reference))
  (bind _returnvalue (Transformation|GetActorRotation))
  (bind _returnvalue_2 (Transformation|GetActorLocation Target))
  ;[1 1 1] Proper Launch
  (Effects|SpawnEmitteratLocation (Variables|Default|GetVFX_LaunchProper) _returnvalue_2)
  (Audio|PlaySoundatLocation (Variables|Default|GetSFX_Nota) _returnvalue_2)
  (bind _output_get (Variables|Default|SetLaunchDirection (Math|Rotator|MakeRotator (.roll _returnvalue) (+ (.pitch _returnvalue) (Variables|Default|GetLaunchPitch)) (.yaw _returnvalue))))
  (bind _output_get_2 (Variables|Default|SetLaunchVelocity (* (Math|Rotator|GetRotationXVector _output_get) (Variables|Default|GetForce))))
  (Character|LaunchCharacter Target _output_get_2 true true))

(event Custom|LaunchPenalty
  (params (Target :type Character%20Object%20Reference))
  (bind _returnvalue (Transformation|GetActorLocation Target))
  (bind _returnvalue_2 (Transformation|GetActorRotation))
  ;[1 1 1] Penalty Launch
  (Effects|SpawnEmitteratLocation (Variables|Default|GetVFX_PenaltyJump) _returnvalue)
  (Audio|PlaySoundatLocation (Variables|Default|GetSFX_NotaPenalty) _returnvalue)
  (bind _output_get (Variables|Default|SetLaunchDirection (Math|Rotator|MakeRotator (.roll _returnvalue_2) (+ (.pitch _returnvalue_2) 1.8e+02) (.yaw _returnvalue_2))))
  (bind _output_get_2 (Variables|Default|SetLaunchVelocity (* (Math|Rotator|GetRotationXVector _output_get) (Math|Random|RandomFloatinRange 6e+02 1e+03))))
  (Character|LaunchCharacter Target _output_get_2 true true))

(event EventBeginPlay
  (bind _staticmesh (Variables|Default|GetStaticMesh))
  ;[1 1 1] Set Color
  (bind _asbp_game_mode (Utilities|Casting|CastToBP_GameMode (Game|GetGameMode)))
  (Variables|Default|SetGameMode _asbp_game_mode)
  (switch Utilities|FlowControl|Switch|SwitchonEnum_Forms (Variables|Default|GetE_Form)
    (:NewEnumerator0
      (Rendering|Material|SetMaterial _staticmesh 0 "/Game/Material/M_Square_Inst.M_Square_Inst")
      (Variables|Default|SetSFX_Nota "/Game/SFX/Cue_Square_impact.Cue_Square_impact"))
    (:NewEnumerator1
      (Rendering|Material|SetMaterial _staticmesh 0 "/Game/Material/M_Circle_Inst.M_Circle_Inst")
      (Variables|Default|SetSFX_Nota "/Game/SFX/Cue_Circle_impact.Cue_Circle_impact"))
    (:NewEnumerator2
      (Rendering|Material|SetMaterial _staticmesh 0 "/Game/Material/M_Triangle_Inst.M_Triangle_Inst")
      (Variables|Default|SetSFX_Nota "/Game/SFX/Cue_Triangle_impact.Cue_Triangle_impact"))
    (:NewEnumerator3
      (Rendering|Material|SetMaterial _staticmesh 0 "/Game/Material/M_Diamond_Inst.M_Diamond_Inst")
      (Variables|Default|SetSFX_Nota "/Game/SFX/Cue_Diamond_impact.Cue_Diamond_impact"))))

(event Collision|EventActorBeginOverlap
  (params (OtherActor :type Actor%20Object%20Reference))
  (bind _gamemode (Variables|Default|GetGameMode))
  (bind _score (Variables|Default|GetScore))
  ;[1 1 1] Overlap
  (bind _asbp_pawn (Utilities|Casting|CastToBP_Pawn OtherActor))
  (if (== (Rendering|Material|GetMaterial (Variables|Default|GetStaticMesh) 0) (Rendering|Material|GetMaterial (Variables|/Script/Engine.Character|GetMesh _asbp_pawn) 0))
    (CallFunction|LaunchProper _asbp_pawn)
    (Default|ScoreSystem _gamemode _score)
    (else
      (CallFunction|LaunchPenalty _asbp_pawn)
      (Default|ScoreSystem _gamemode (* _score -1)))))

(fn ConstructionScript
  (Variables|Default|SetE_Form (Utilities|Enum|ByteToEnumEnum_Forms (Math|Conversions|ToByte(Integer) (Math|Random|RandomIntegerinRange 0 3)))))