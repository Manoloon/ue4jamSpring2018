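; BP_Segment is a level segment that fills itself with platforms and chains the next segment as the pawn passes through.
; Its construction script scatters 16 child actors at random points inside the SpawnPlatforms box.
; A pawn overlapping Out asks BP_GameMode to spawn another segment, then this one destroys itself after a short delay.
; A pawn overlapping Killzone is destroyed.
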(event OnComponentBeginOverlap(Out)
  (params (OverlappedComponent :type Primitive%20Component%20Object%20Reference) (OtherActor :type Actor%20Object%20Reference) (OtherComp :type Primitive%20Component%20Object%20Reference) (OtherBodyIndex :type Integer) (bFromSweep :type Boolean) (SweepResult :type Hit%20Result%20Structure%20%28by%20ref%29))
  (Utilities|Casting|CastToBP_Pawn OtherActor)
  (Default|SpawnSegment (Variables|Default|GetGameMode))
  (Utilities|FlowControl|Delay 3.0)
  (Actor|DestroyActor))

(event OnComponentBeginOverlap(Killzone)
  (params (OverlappedComponent :type Primitive%20Component%20Object%20Reference) (OtherActor :type Actor%20Object%20Reference) (OtherComp :type Primitive%20Component%20Object%20Reference) (OtherBodyIndex :type Integer) (bFromSweep :type Boolean) (SweepResult :type Hit%20Result%20Structure%20%28by%20ref%29))
  (bind _asbp_pawn (Utilities|Casting|CastToBP_Pawn OtherActor))
  (Actor|DestroyActor _asbp_pawn))

(event EventBeginPlay
  (bind _asbp_game_mode (Utilities|Casting|CastToBP_GameMode (Game|GetGameMode)))
  (Variables|Default|SetGameMode _asbp_game_mode))

(event Collision|EventActorBeginOverlap
  (params (OtherActor :type Actor%20Object%20Reference)))

(event EventTick
  (params (DeltaSeconds :type Float%20%28single-precision%29)))

(fn ConstructionScript
  (bind _spawnplatforms (Variables|Default|GetSpawnPlatforms))
  (for _index (range 0 15)
    (AddComponent|AddChildActorComponent true (Math|Transform|MakeTransform (Math|Random|RandomPointinBoundingBox (Transformation|GetWorldLocation _spawnplatforms) (Components|Box|GetScaledBoxExtent _spawnplatforms)) "0, 0, 0" "1,1,1"))))