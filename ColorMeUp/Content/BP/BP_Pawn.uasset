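; BP_Pawn is the player pawn, moved along world X and Y by axis inputs and able to switch between four shape-named materials.
; Square, Triangle, Circle and Diamond inputs set the mesh material and share one ten-second Delay before restoring the default, so later presses don't restart the countdown.
; BeginPlay caches BP_GameMode and activates the camera.
; On destruction it plays a death sound and calls PlayerDeath on the game mode.
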(event EventBeginPlay
  ;[1 1 1] Begin play
  (bind _asbp_game_mode (Utilities|Casting|CastToBP_GameMode (Game|GetGameMode)))
  (Variables|Default|SetGameMode _asbp_game_mode)
  (Components|Activation|SetActive (Variables|Default|GetCamera) true false))

(event EventDestroyed
  ;[1 1 1] Death
  (Audio|PlaySound2D "/Game/SFX/Cue_Die.Cue_Die")
  (Default|PlayerDeath (Variables|Default|GetGameMode)))

(event Input|ActionEvents|InputActionSquare
  (params (Key :type Key%20Structure))
  (bind _mesh (Variables|Character|GetMesh))
  (:Pressed
    (Rendering|Material|SetMaterial _mesh 0 "/Game/Material/M_Square_Inst.M_Square_Inst")
    (Utilities|FlowControl|Delay 1e+01)
    (Rendering|Material|SetMaterial _mesh 0 "/Engine/EngineMaterials/DefaultMaterial.DefaultMaterial")))

(event Input|ActionEvents|InputActionTriangle
  (params (Key :type Key%20Structure))
  (bind _mesh (Variables|Character|GetMesh))
  (:Pressed
    (Rendering|Material|SetMaterial _mesh 0 "/Game/Material/M_Triangle_Inst.M_Triangle_Inst")
    (Utilities|FlowControl|Delay 1e+01)
    (Rendering|Material|SetMaterial _mesh 0 "/Engine/EngineMaterials/DefaultMaterial.DefaultMaterial")))

(event Input|ActionEvents|InputActionCircle
  (params (Key :type Key%20Structure))
  (bind _mesh (Variables|Character|GetMesh))
  (:Pressed
    (Rendering|Material|SetMaterial _mesh 0 "/Game/Material/M_Circle_Inst.M_Circle_Inst")
    (Utilities|FlowControl|Delay 1e+01)
    (Rendering|Material|SetMaterial _mesh 0 "/Engine/EngineMaterials/DefaultMaterial.DefaultMaterial")))

(event Input|ActionEvents|InputActionDiamond
  (params (Key :type Key%20Structure))
  (bind _mesh (Variables|Character|GetMesh))
  (:Pressed
    (Rendering|Material|SetMaterial _mesh 0 "/Game/Material/M_Diamond_Inst.M_Diamond_Inst")
    (Utilities|FlowControl|Delay 1e+01)
    (Rendering|Material|SetMaterial _mesh 0 "/Engine/EngineMaterials/DefaultMaterial.DefaultMaterial")))

(event Input|AxisEvents|InputAxisMoveRight
  (params (AxisValue :type Float%20%28single-precision%29))
  ;[1 1 1] Movement
  (Pawn|Input|AddMovementInput "0.000000,1.000000,0.000000" AxisValue false))

(event Input|AxisEvents|InputAxisMoveForward
  (params (AxisValue :type Float%20%28single-precision%29))
  ;[1 1 1] Movement
  (Pawn|Input|AddMovementInput "1.000000,0.000000, 0" AxisValue false))

(fn ConstructionScript)