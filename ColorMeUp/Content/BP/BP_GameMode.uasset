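; Game mode for a segment-based level that manages the HUD, score, persistent high score, game over and player death.
; BeginPlay loads or creates the high-score save, starts the HUD, then chains initial segments, spawning each at the previous one's PuntoAncla anchor.
; Score updates save any new high score immediately.
; Game over destroys the pawn, while player death blends to BP_WinCamera before opening M_Level4.
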(event Custom|ScoreSystem
  (params (A :type Integer))
  ;[1 1 1] Score
  (bind _output_get (Variables|Default|SetScore (+ A (Variables|Default|GetScore))))
  (if (> _output_get (Variables|Default|GetHiscore))
    (bind _output_get_2 (Variables|Default|SetHiscore _output_get))
    (CallFunction|SaveHiscoreEVent _output_get_2))
  (Default|WGScoreText (Variables|Default|GetGameHud_Ref) (Variables|Default|GetScore)))

(event Custom|PlayerDeath
  ;[1 1 1] Player Death
  (bind _outactors (Actor|GetAllActorsOfClass "/Game/BP/BP_WinCamera.BP_WinCamera_C"))
  (Utilities|IsValid (Utilities|Array|Get(acopy) _outactors)
    (:Is%20Valid
      (Game|Player|SetViewTargetwithBlend (Game|GetPlayerController 0) (Utilities|Array|Get(acopy) _outactors) 3.0 "VTBlend_Cubic" 0.0 false)
      (Default|WGStartGame (Variables|Default|GetGameHud_Ref) false)
      (Utilities|FlowControl|Delay 3.0)
      (Game|OpenLevel(byName) "M_Level4"))))

(event Custom|GameOverEvent
  ;[1 1 1] Game over event
  (bind _outactors (Actor|GetAllActorsOfClass "/Game/BP/BP_Pawn.BP_Pawn_C"))
  (Actor|DestroyActor (Utilities|Array|Get(acopy) _outactors))
  (Variables|Default|SetbIsGameOver true)
  (Default|WGStageEvent (Variables|Default|GetGameHud_Ref) false))

(event Custom|SaveHiscore%20EVent
  (params (Hiscore :type Integer))
  ;[1 1 1] Hiscore
  (bind _assg_hiscore (Utilities|Casting|CastToSG_Hiscore (Variables|Default|GetHiscoreSave)))
  (Utilities|IsValid _assg_hiscore
    (:Is%20Valid
      (Variables|/Game/BP/SG_Hiscore.SG_Hiscore_C|SetHiscore _assg_hiscore Hiscore)
      (SaveGame|SaveGametoSlot _assg_hiscore (Variables|Default|GetHiscoreName))
      (Default|WGHiscore (Variables|Default|GetGameHud_Ref) (Variables|Default|GetHiscore)))
    (:Is%20Not%20Valid
      (Development|PrintString "Failed HISCORE"))))

(event Custom|SpawnSegment
  ;[1 1 1] Spawn Segmentos
  (bind _returnvalue (Game|SpawnActorfromClass "/Game/BP/BP_Segment.BP_Segment_C" (Math|Transform|MakeTransform (Variables|Default|GetNextSegment) "0, 0, 0" "1,1,1") "AlwaysSpawn" 0 0))
  (Variables|Default|SetNextSegment (Transformation|GetWorldLocation (Variables|/Game/BP/BP_Segment.BP_Segment_C|GetPuntoAncla _returnvalue))))

(event Custom|SpawnCoins)

(event Custom|StartGame%20Event
  (bind _returnvalue (Game|GetPlayerController 0))
  ;[1 1 1] STart Game event
  (Variables|/Script/Engine.PlayerController|SetbShowMouseCursor _returnvalue false)
  (bind _returnvalue_2 (UserInterface|CreateWidget "/Game/HUD/WG_Gameplay.WG_Gameplay_C" _returnvalue))
  (bind _output_get (Variables|Default|SetGameHud_Ref _returnvalue_2))
  (UserInterface|Viewport|AddtoViewport _output_get 0)
  (CallFunction|ScoreSystem (Variables|Default|GetScore))
  (CallFunction|LoadHiscoreEvent)
  (Utilities|FlowControl|Delay 3.0)
  (Default|WGStartGame (Variables|Default|GetGameHud_Ref) true))

(event Custom|LoadHiscore%20Event
  ;[1 1 1] Hiscore
  (bind _assg_hiscore (Utilities|Casting|CastToSG_Hiscore (Variables|Default|GetHiscoreSave)))
  (SaveGame|LoadGamefromSlot (Variables|Default|GetHiscoreName))
  (Utilities|IsValid _assg_hiscore
    (:Is%20Valid
      (bind _output_get (Variables|Default|SetHiscore (Variables|/Game/BP/SG_Hiscore.SG_Hiscore_C|GetHiscore _assg_hiscore)))
      (Default|WGHiscore (Variables|Default|GetGameHud_Ref) _output_get))
    (:Is%20Not%20Valid
      (Development|PrintString "Failed HISCORE"))))

(event EventBeginPlay
  ;[1 1 1] BeginPlay
  (bind _returnvalue (SaveGame|DoesSaveGameExist (Variables|Default|GetHiscoreName)))
  (if _returnvalue
    (bind _returnvalue_2 (SaveGame|LoadGamefromSlot (Variables|Default|GetHiscoreName)))
    (bind _output_get (Variables|Default|SetHiscoreSave _returnvalue_2))
    (bind _assg_hiscore (Utilities|Casting|CastToSG_Hiscore _output_get))
    (Variables|Default|SetHiscore (Variables|/Game/BP/SG_Hiscore.SG_Hiscore_C|GetHiscore _assg_hiscore))
    (else
      (bind _returnvalue_3 (SaveGame|CreateSaveGameObject "/Game/BP/SG_Hiscore.SG_Hiscore_C"))
      (bind _output_get_2 (Variables|Default|SetHiscoreSave _returnvalue_3))
      (Utilities|Casting|CastToSG_Hiscore _output_get_2)))
  (CallFunction|StartGameEvent)
  (for _index (range 0 4)
    (CallFunction|SpawnSegment)))

(fn ConstructionScript)