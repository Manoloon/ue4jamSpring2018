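; BP_Cells is a rotating shape cell that lets a BP_Pawn with a matching material through and blocks one that differs.
; BeginPlay applies the square, circle, triangle or diamond material from EForm, and material equality serves as the shape test.
; On overlap it records the pawn as Friendly or Enemy, switches the box collision accordingly, then restores overlap after a short delay.
; The construction script randomly keeps, reverses or zeroes yaw spin.
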(event EventBeginPlay
  (bind _staticmesh (Variables|Default|GetStaticMesh))
  (switch Utilities|FlowControl|Switch|SwitchonEnum_Forms (Variables|Default|GetE_Form)
    (:NewEnumerator0
      (Rendering|Material|SetMaterial _staticmesh 0 "/Game/Material/M_Square_Inst.M_Square_Inst"))
    (:NewEnumerator1
      (Rendering|Material|SetMaterial _staticmesh 0 "/Game/Material/M_Circle_Inst.M_Circle_Inst"))
    (:NewEnumerator2
      (Rendering|Material|SetMaterial _staticmesh 0 "/Game/Material/M_Triangle_Inst.M_Triangle_Inst"))
    (:NewEnumerator3
      (Rendering|Material|SetMaterial _staticmesh 0 "/Game/Material/M_Diamond_Inst.M_Diamond_Inst"))))

(event Collision|EventActorBeginOverlap
  (params (OtherActor :type Actor%20Object%20Reference))
  (bind _box (Variables|Default|GetBox))
  (bind _asbp_pawn (Utilities|Casting|CastToBP_Pawn OtherActor))
  (if (== (Rendering|Material|GetMaterial (Variables|/Script/Engine.Character|GetMesh _asbp_pawn) 0) (Rendering|Material|GetMaterial (Variables|Default|GetStaticMesh) 0))
    (Variables|Default|SetFriendly OtherActor)
    (Collision|SetCollisionProfileName _box "NoCollision" :!class /Script/Engine.PrimitiveComponent)
    (else
      (Variables|Default|SetEnemy OtherActor)
      (Collision|SetCollisionProfileName _box "BlockAll" :!class /Script/Engine.PrimitiveComponent)))
  (Utilities|FlowControl|Delay 2.0)
  (Collision|SetCollisionProfileName _box "OverlapAllDynamic" :!class /Script/Engine.PrimitiveComponent))

(event EventTick
  (params (DeltaSeconds :type Float%20%28single-precision%29)))

(fn ConstructionScript
  (bind _rotatingmovement (Variables|Default|GetRotatingMovement))
  (Variables|/Script/Engine.RotatingMovementComponent|SetRotationRate _rotatingmovement (Math|Rotator|MakeRotator (.roll (Variables|/Script/Engine.RotatingMovementComponent|GetRotationRate _rotatingmovement)) (.pitch (Variables|/Script/Engine.RotatingMovementComponent|GetRotationRate _rotatingmovement)) (* (Math|Random|RandomIntegerinRange -1 1) (.yaw (Variables|/Script/Engine.RotatingMovementComponent|GetRotationRate _rotatingmovement))))))